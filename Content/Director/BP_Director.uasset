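; BP_Director manages the zombie population, tracking live zombies and fulfilling horde spawner requests.
; On BeginPlay it registers existing zombies and horde spawners, binding to their killed and spawn-request events.
; Spawn requests are capped by MaxZombies and place zombies at random reachable navmesh points near the requested location, adjusting for collision or skipping blocked spawns.
; Newly spawned zombies are registered through the same path as pre-placed ones.
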(event EventBeginPlay
  (Utilities|FlowControl|Sequence
    (:then_0
      (bind _outactors (Actor|GetAllActorsOfClass "/Game/GameFiles/Zombie/Blueprints/BP_zombie.BP_zombie_C"))
      (for _array_element _outactors
        (Private|OnZombieSpawned _array_element)))
    (:then_1
      (bind _outactors_2 (Actor|GetAllActorsOfClass "/Game/Director/BP_HordeSpawner.BP_HordeSpawner_C"))
      (for _array_element_2 _outactors_2
        (Private|OnHordeSpawnerSpawned _array_element_2)))))

(fn ConstructionScript)

(fn OnZombieSpawned
  (params (Zombie :type BP%20Zombie%20Object%20Reference))
  (Utilities|Array|Add (Variables|Default|GetZombies) Zombie)
  (EventDispatchers|BindEventtoOnKilled Zombie (EventDispatchers|CreateEvent :!event OnZombieKilled)))

(fn OnZombieKilled
  (params (Zombie :type BP%20Zombie%20Object%20Reference))
  (Utilities|Array|RemoveItem (Variables|Default|GetZombies) Zombie))

(fn OnHordeSpawnerSpawned
  (params (HordeSpawner :type BP%20Horde%20Spawner%20Object%20Reference))
  (Utilities|Array|Add (Variables|Default|GetHordeSpawners) HordeSpawner)
  (EventDispatchers|BindEventtoRequestSpawn HordeSpawner (EventDispatchers|CreateEvent :!event OnZombieSpawnRequested)))

(fn OnZombieSpawnRequested
  (params (Count :type Integer) (Location :type Vector))
  (for _index (range 1 (Math|Integer|Min(Integer) Count (- (Variables|Default|GetMaxZombies) (Utilities|Array|Length (Variables|Default|GetZombies)))))
    (bind _returnvalue (Game|SpawnActorfromClass "/Game/GameFiles/Zombie/Blueprints/BP_zombie.BP_zombie_C" (Math|Transform|MakeTransform (+ (.RandomLocation (AI|Navigation|GetRandomReachablePointinRadius Location 2e+02 0 0)) "0, 0,88.000000") "0, 0, 0" "1,1,1") "AdjustIfPossibleButDontSpawnIfColliding" 0 0))
    (Utilities|IsValid _returnvalue
      (:Is%20Valid
        (Private|OnZombieSpawned _returnvalue)))))