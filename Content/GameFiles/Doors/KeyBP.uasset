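; KeyBP is a key pickup that the player collects with the Interact input while standing in its box trigger.
; Overlap by a Ue4ASP_Character enables input and opens a gate, and end overlap reverses both.
; Interacting through the open gate sets HasKey on the character, plays a sound and destroys the key.
; The widget shows and hides on overlap by any actor, as that branch skips the cast.
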(event OnComponentBeginOverlap(Box)
  (params (OverlappedComponent :type Primitive%20Component%20Object%20Reference) (OtherActor :type Actor%20Object%20Reference) (OtherComp :type Primitive%20Component%20Object%20Reference) (OtherBodyIndex :type Integer) (bFromSweep :type Boolean) (SweepResult :type Hit%20Result%20Structure%20%28by%20ref%29))
  (Utilities|FlowControl|Sequence
    (:then_0
      (bind _asue_4asp_character (Utilities|Casting|CastToUe4ASP_Character OtherActor))
      (Input|EnableInput (Game|GetPlayerController 0))
      (Utilities|FlowControl|Gate true) ; enters at Open
    )
    (:then_1
      (Development|SetHiddeninGame (Variables|Default|GetWidget) false false))))

(event OnComponentEndOverlap(Box)
  (params (OverlappedComponent :type Primitive%20Component%20Object%20Reference) (OtherActor :type Actor%20Object%20Reference) (OtherComp :type Primitive%20Component%20Object%20Reference) (OtherBodyIndex :type Integer))
  (Utilities|FlowControl|Sequence
    (:then_0
      (Utilities|Casting|CastToUe4ASP_Character OtherActor)
      (Input|DisableInput (Game|GetPlayerController 0))
      (Utilities|FlowControl|Gate true) ; enters at Close
    )
    (:then_1
      (Development|SetHiddeninGame (Variables|Default|GetWidget) true false))))

(event Input|ActionEvents|InputActionInteract
  (params (Key :type Key%20Structure :default "None"))
  (:Pressed
    (Utilities|FlowControl|Gate true
      (:Exit
        (Variables|/Game/GameFiles/Character/Ue4ASP_Character.Ue4ASP_Character_C|SetHasKey? (stale OnComponentBeginOverlap(Box) _asue_4asp_character) true)
        (Audio|PlaySoundatLocation "/Game/GameFiles/Sounds/Inspect.Inspect" (Transformation|GetActorLocation) "0, 0, 0" 1.0 1.0 0.0 0 0 0)
        (Actor|DestroyActor)))))

(fn ConstructionScript)