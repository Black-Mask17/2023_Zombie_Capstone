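; Bullet actor from the gun that kills zombies it hits.
; The Hit event tries casts to BP_zombie, BP_zombie1 and BP_zombie2 in turn and calls Kill on the first match.
; Disconnected leftover logic holds Enemy tag checks and DestroyActor calls, so the live graph neither filters by tag nor destroys the bullet.
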(event Collision|EventHit
  (params (MyComp :type Primitive%20Component%20Object%20Reference) (Other :type Actor%20Object%20Reference) (OtherComp :type Primitive%20Component%20Object%20Reference) (bSelfMoved :type Boolean) (HitLocation :type Vector :default "0, 0, 0") (HitNormal :type Vector :default "0, 0, 0") (NormalImpulse :type Vector :default "0, 0, 0") (Hit :type Hit%20Result%20Structure%20%28by%20ref%29))
  (bind _asbp_zombie (Utilities|Casting|CastToBP_zombie Other)
    (:then
      (Default|Kill _asbp_zombie))
    (:CastFailed
      (bind _asbp_zombie_1 (Utilities|Casting|CastToBP_zombie1 Other)
        (:then
          (Default|Kill _asbp_zombie_1))
        (:CastFailed
          (bind _asbp_zombie_2 (Utilities|Casting|CastToBP_zombie2 Other))
          (Default|Kill _asbp_zombie_2))))))

(fn ConstructionScript)