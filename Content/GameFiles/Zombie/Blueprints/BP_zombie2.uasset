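; Zombie enemy character that randomizes its scale, facing and walk speed on spawn and registers with the game mode's alive count.
; Pawn sensing triggers a sound and a repeating AIMoveTo chase of the player.
; Box overlap plays an attack montage once per entry, with damage applied through a separate DamagePlayer event.
; Kill stops AI logic, ragdolls the mesh, credits a kill, then after a delay decrements the count and destroys the actor.
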(event OnSeePawn(PawnSensing)
  (params (Pawn :type Pawn%20Object%20Reference))
  (bind _asue_4asp_character (Utilities|Casting|CastToUe4ASP_Character Pawn))
  (Utilities|FlowControl|Sequence
    (:then_0
      (Utilities|FlowControl|Sequence
        (:then_0
          (Utilities|FlowControl|DoOnce false :!label _label
            (:Completed
              (Audio|PlaySoundatLocation "/Game/GameFiles/Sounds/Zombie_Cue_2.Zombie_Cue_2" (Transformation|GetActorLocation) "0, 0, 0" 1.0 1.0 0.0 0 0 0))))
        (:then_1
          (Utilities|FlowControl|RetriggerableDelay 1.0)
          (goto _label Reset))))
    (:then_1
      (CallFunction|ChasePlayer _asue_4asp_character))))

(event OnComponentBeginOverlap(Box)
  (params (OverlappedComponent :type Primitive%20Component%20Object%20Reference) (OtherActor :type Actor%20Object%20Reference) (OtherComp :type Primitive%20Component%20Object%20Reference) (OtherBodyIndex :type Integer) (bFromSweep :type Boolean) (SweepResult :type Hit%20Result%20Structure%20%28by%20ref%29))
  (bind _asue_4asp_character (Utilities|Casting|CastToUe4ASP_Character OtherActor))
  (Variables|Default|SetPlayer _asue_4asp_character)
  (Utilities|FlowControl|DoOnce false
    (:Completed
      (Animation|Montage|MontagePlay (Components|SkeletalMesh|GetAnimInstance (Variables|Character|GetMesh)) "/Game/GameFiles/Zombie/Resource/Zombie_Attack_Montage.Zombie_Attack_Montage" 1.0 "MontageLength" 0.0 true))))

(event OnComponentEndOverlap(Box)
  (params (OverlappedComponent :type Primitive%20Component%20Object%20Reference) (OtherActor :type Actor%20Object%20Reference) (OtherComp :type Primitive%20Component%20Object%20Reference) (OtherBodyIndex :type Integer))
  (Utilities|Casting|CastToUe4ASP_Character OtherActor)
  (CallFunction|Reset))

(event Custom|Kill
  (bind _mesh (Variables|Character|GetMesh))
  (AI|Logic|StopLogic (Variables|/Script/AIModule.AIController|GetBrainComponent (AI|GetAIController self)) "")
  (Collision|SetCollisionProfileName _mesh "Ragdoll" true :!class /Script/Engine.PrimitiveComponent)
  (Physics|SetSimulatePhysics _mesh true)
  (Collision|SetCollisionProfileName (Variables|Collision|GetCapsuleComponent) "No Collision" true :!class /Script/Engine.PrimitiveComponent)
  (Utilities|FlowControl|Sequence
    (:then_0
      (bind _asue_4asp_character (Utilities|Casting|CastToUe4ASP_Character (Game|GetPlayerCharacter 0)))
      (Math|Integer|IncrementInt (Variables|/Game/GameFiles/Character/Ue4ASP_Character.Ue4ASP_Character_C|GetKills _asue_4asp_character)))
    (:then_1
      (Utilities|FlowControl|Delay 1.0)
      (Default|CallOnKilled self)
      (Utilities|Casting|CastToUe4ASP_Character (Game|GetPlayerCharacter 0))
      (bind _asthird_person_game_mode (Utilities|Casting|CastToThirdPersonGameMode (Game|GetGameMode)))
      (Variables|/Game/ThirdPersonBP/Blueprints/ThirdPersonGameMode.ThirdPersonGameMode_C|SetAmount%20Alive%20End _asthird_person_game_mode (- (Variables|/Game/ThirdPersonBP/Blueprints/ThirdPersonGameMode.ThirdPersonGameMode_C|GetAmount%20Alive%20End _asthird_person_game_mode) 1))
      (Actor|DestroyActor))))

(event Custom|ChasePlayer
  (params (PlayerTOChase :type Pawn%20Object%20Reference))
  (AI|AIMoveTo self "0, 0, 0" PlayerTOChase 5.0 false
    (:then
      (Utilities|FlowControl|Delay 1.0)
      (CallFunction|ChasePlayer PlayerTOChase))))

(event Custom|Reset
  (Utilities|FlowControl|DoOnce false) ; enters at Reset
)

(event Custom|DamagePlayer
  (Game|Damage|ApplyDamage (Variables|Default|GetPlayer) (Variables|Default|GetDamage) 0 self))

(event EventBeginPlay
  (bind _returnvalue (Math|Random|RandomFloatinRange 0.9 1.1))
  (Utilities|FlowControl|Sequence
    (:then_0
      (Transformation|SetWorldScale3D (Variables|Character|GetMesh) (Math|Vector|MakeVector _returnvalue _returnvalue _returnvalue))
      (Transformation|SetActorRotation (Math|Rotator|MakeRotator 0.0 0.0 (Math|Random|RandomFloatinRange 0.0 3.6e+02)))
      (Variables|/Script/Engine.CharacterMovementComponent|SetMaxWalkSpeed (Variables|Character|GetCharacterMovement) (Math|Random|RandomFloatinRange 4.5e+02 6e+02)))
    (:then_1
      (bind _asthird_person_game_mode (Utilities|Casting|CastToThirdPersonGameMode (Game|GetGameMode)))
      (Variables|/Game/ThirdPersonBP/Blueprints/ThirdPersonGameMode.ThirdPersonGameMode_C|SetAmount%20Alive%20End _asthird_person_game_mode (+ (Variables|/Game/ThirdPersonBP/Blueprints/ThirdPersonGameMode.ThirdPersonGameMode_C|GetAmount%20Alive%20End _asthird_person_game_mode) 1)))))

(fn ConstructionScript)